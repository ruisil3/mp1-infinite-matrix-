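; Projectile actor that destroys enemies it hits and awards score to the player.
; Tick moves the Sphere component along its local X axis by a frame-rate-independent offset, at a speed SetProjectileSpeed sets to double the given player speed.
; An overlap on the Collision component with an Enemy destroys that enemy and increases the Player's score, without destroying the projectile.
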(event `self.ReceiveTick`
  (params (DeltaSeconds :type "Float (single-precision)"))
  (`SceneComponent.K2_AddLocalOffset` (`self.Sphere`) (`KismetMathLibrary.MakeVector` (* DeltaSeconds (`self.ProjectileSpeed`))) false false))

(event `self.Collision.OnComponentBeginOverlap`
  (params (OverlappedComponent :type "PrimitiveComponent Object Reference") (OtherActor :type "Actor Object Reference") (OtherComp :type "PrimitiveComponent Object Reference") (OtherBodyIndex :type Integer) (bFromSweep :type Boolean) (SweepResult :type "HitResult Structure (by ref)"))
  (bind _player (`self.Player`))
  (bind _asenemy (cast `/Game/InfiniteMatrix/Blueprints/Enemy` OtherActor))
  (`self.K2_DestroyActor` _asenemy)
  (set `/Game/InfiniteMatrix/Blueprints/BP_Player.Score` (+ (`/Game/InfiniteMatrix/Blueprints/BP_Player.Score` _player) 20) _player))

(fn `SetProjectileSpeed`
  (params (PlayerSpeed :type "Float (double-precision)"))
  (set `self.ProjectileSpeed` (* PlayerSpeed 2.0)))

(fn `UserConstructionScript`)